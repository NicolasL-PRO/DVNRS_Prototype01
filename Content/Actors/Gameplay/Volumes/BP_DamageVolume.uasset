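; BP_DamageVolume is a switchable volume that repeatedly damages overlapping actors of allowed classes, with an optional fog visual.
; Overlap begin starts a looping ApplyDamage timer and maps the actor to its handle; overlap end clears it.
; ApplyDamage reads one shared ActorToDamage, so it targets only the latest entrant.
; The construction script sizes volume and fog cube, while a looping timeline animates the fog's dynamic material.
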(event `self.ReceiveBeginPlay`
  (bind _fogdensity (`self.FogDensity`))
  (bind _emissivestrength (`self.EmissiveStrength`))
  (bind _animationplayrate (`self.AnimationPlayRate`))
  (`BlueprintMapLibrary.Map_Clear` (`self.ActorsToDamage`))
  (`KismetSystemLibrary.K2_ClearTimer` null "ApplyDamage")
  (if (and (`self.UseFog?`) (`self.UseAnimation?`))
    (`TimelineComponent.SetPlayRate` (`self.FogAnimation`) (`KismetMathLibrary.SelectFloat` 1.0 _animationplayrate (== _animationplayrate 0.0)) :!label _label)
    (bind (_direction _densityalpha _emissivealpha) (`Timeline|FogAnimation` :!via `PlayFromStart`)
      (:`Update`
        (`MaterialInstanceDynamic.SetScalarParameterValue` (`self.MaterialInstance`) "EmissiveStrength" (`KismetMathLibrary.Lerp` _emissivestrength (* _emissivestrength 0.0) _densityalpha))
        (`MaterialInstanceDynamic.SetScalarParameterValue` (`self.MaterialInstance`) "FogDensity" (`KismetMathLibrary.Lerp` (* _fogdensity 0.0) _fogdensity _emissivealpha)))
      (:`Finished`
        (goto _label)))))

(event `DamageVolume_Switch_Event`
  (params (`On?` :type Boolean))
  (set `self.TurnedOn?` `On?`))

(event `self.DamageVolume.OnComponentBeginOverlap`
  (params (OverlappedComponent :type "PrimitiveComponent Object Reference") (OtherActor :type "Actor Object Reference") (OtherComp :type "PrimitiveComponent Object Reference") (OtherBodyIndex :type Integer) (bFromSweep :type Boolean) (SweepResult :type "HitResult Structure (by ref)"))
  (bind _every (`self.Every`))
  (if (`self.TurnedOn?`)
    (if (`BlueprintMapLibrary.Map_Contains` (`self.CastDamageTo`) (`GameplayStatics.GetObjectClass` OtherActor))
      (if (not (`BlueprintMapLibrary.Map_Contains` (`self.ActorsToDamage`) OtherActor))
        (set `self.ActorToDamage` OtherActor)
        (bind _returnvalue (`KismetSystemLibrary.K2_SetTimer` null "ApplyDamage" _every true false (- 0.0 _every)))
        (`BlueprintMapLibrary.Map_Add` (`self.ActorsToDamage`) OtherActor _returnvalue)))))

(event `self.DamageVolume.OnComponentEndOverlap`
  (params (OverlappedComponent :type "PrimitiveComponent Object Reference") (OtherActor :type "Actor Object Reference") (OtherComp :type "PrimitiveComponent Object Reference") (OtherBodyIndex :type Integer))
  (if (`self.TurnedOn?`)
    (`KismetSystemLibrary.K2_ClearAndInvalidateTimerHandle` (`BlueprintMapLibrary.Map_Find` (`self.ActorsToDamage`) OtherActor))
    (`BlueprintMapLibrary.Map_Remove` (`self.ActorsToDamage`) OtherActor)))

(event `ApplyDamage`
  (bind _actortodamage (`self.ActorToDamage`))
  (bind _returnvalue (* (`self.DamageAmount`) (`self.DamageFactor`)))
  (`GameplayStatics.ApplyDamage` _actortodamage _returnvalue null self)
  (if (`self.Debug_PrintDamages?`)
    (`KismetSystemLibrary.PrintString` (`KismetStringLibrary.Concat_StrStr` "Applied " (`KismetStringLibrary.Conv_DoubleToString` _returnvalue) " damage to " (`KismetSystemLibrary.GetDisplayName` _actortodamage)) true true (struct :`R` 1.0 :`G` 0.031556 :`A` 1.0) 4.0)))

(fn `UserConstructionScript`
  (locals (NewLocalVar :type "MaterialInstanceDynamic Object Reference"))
  (if (`self.UseFog?`)
    (bind _returnvalue (`PrimitiveComponent.CreateDynamicMaterialInstance` (`self.Cube`) 0 null "None"))
    (bind _output_get (set `self.MaterialInstance` _returnvalue))
    (`PrimitiveComponent.SetMaterial` (`self.Cube`) 0 _output_get)
    (`MaterialInstanceDynamic.SetVectorParameterValue` (`self.MaterialInstance`) "FogColor" (`self.FogColor`))
    (`MaterialInstanceDynamic.SetScalarParameterValue` (`self.MaterialInstance`) "EmissiveStrength" (`self.EmissiveStrength`))
    (`MaterialInstanceDynamic.SetScalarParameterValue` (`self.MaterialInstance`) "FogDensity" (`self.FogDensity`))
    (`SceneComponent.SetWorldScale3D` (`self.Cube`) (`self.DamageVolumeScale`))
    (else
      (`PrimitiveComponent.SetMaterial` (`self.Cube`) 0 null)
      (`SceneComponent.SetWorldScale3D` (`self.Cube`) (0.0 0.0 0.0))))
  (`SceneComponent.SetWorldScale3D` (`self.DamageVolume`) (`self.DamageVolumeScale`))
  (`SceneComponent.SetHiddenInGame` (`self.DamageVolume`) (not (`self.VolumeVisibleInGame?`)) false))