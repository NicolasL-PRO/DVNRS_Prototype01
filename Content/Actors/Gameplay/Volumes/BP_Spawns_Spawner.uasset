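; Spawner volume that, on a spawn call, creates AI of a chosen class at random points inside a configurable box, facing a set direction.
; After an initial delay it makes one attempt per requested entity, destroying any that overlap static mesh actors without retrying.
; Optionally, it then messages the survivors to play their behaviour, staggered by a delayed loop with optional randomised timing.
; Reset clears the entity list and flags spawning to stop.
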(event `/Game/TPS_Game/Blueprints/System/BPI_IaControls.IA_Reset`
  (bind (_spawndata_spawn_delaybeforespawnstart _spawndata_spawn_amountofentities) (break `/Game/TPS_Game/Blueprints/System/S_IaSpawnData` (`self.SpawnData`)))
  (bind (_spawndata_spawn_delaybeforespawnstart_2 _spawndata_spawn_amountofentities_2 _spawndata_behaviour_playonspawn_) (break `/Game/TPS_Game/Blueprints/System/S_IaSpawnData` (`self.SpawnData`)))
  (bind (_origin _boxextent) (`KismetSystemLibrary.GetComponentBounds` (`self.Spawn_Zone`)))
  (bind _returnvalue (* 0.0 (.y _boxextent)))
  (bind _returnvalue_2 (* 0.0 (.x _boxextent)))
  (`KismetArrayLibrary.Array_Clear` (`self.Entities`))
  (set `self.BreakSpawnLoop` true)
  (goto _label :!via `Break`))

(event `/Game/TPS_Game/Blueprints/System/BPI_IaControls.IA_Spawn`
  (bind (_spawndata_spawn_delaybeforespawnstart _spawndata_spawn_amountofentities) (break `/Game/TPS_Game/Blueprints/System/S_IaSpawnData` (`self.SpawnData`)))
  (bind _spawndata_spawn_delaybeforespawnstart_2 (break `/Game/TPS_Game/Blueprints/System/S_IaSpawnData` (`self.SpawnData`)))
  (bind (_spawndata_spawn_delaybeforespawnstart_3 _spawndata_spawn_amountofentities_2 _spawndata_behaviour_playonspawn_) (break `/Game/TPS_Game/Blueprints/System/S_IaSpawnData` (`self.SpawnData`)))
  (bind (_origin _boxextent) (`KismetSystemLibrary.GetComponentBounds` (`self.Spawn_Zone`)))
  (bind _returnvalue (* 0.0 (.y _boxextent)))
  (bind _returnvalue_2 (* 0.0 (.x _boxextent)))
  (`KismetArrayLibrary.Array_Clear` (`self.Entities`))
  (set `self.BreakSpawnLoop` false)
  (`KismetSystemLibrary.Delay` _spawndata_spawn_delaybeforespawnstart_2)
  (for _ (range (+ _spawndata_spawn_amountofentities 1)) :!label _label
    (if (not (== (`KismetArrayLibrary.Array_Length` (`self.Entities`)) _spawndata_spawn_amountofentities))
      (if (not (`self.BreakSpawnLoop`))
        (bind _returnvalue_3 (`AIBlueprintHelperLibrary.SpawnAIFromClass` (`self.ClassToSpawn`) null (`KismetMathLibrary.TransformLocation` (`self.GetTransform` self) (`KismetMathLibrary.MakeVector` (`KismetMathLibrary.RandomFloatInRange` (* _returnvalue_2 -1.0) _returnvalue_2) (`KismetMathLibrary.RandomFloatInRange` (* _returnvalue -1.0) _returnvalue))) (`SceneComponent.K2_GetComponentRotation` (`self.Spawn_Direction`)) false null))
        (bind _output_get (set `self.Entity` _returnvalue_3))
        (if (`KismetSystemLibrary.IsValid` _output_get)
          (if (> (`KismetArrayLibrary.Array_Length` (`self.GetOverlappingActors` (`self.Entity`) "/Script/Engine.StaticMeshActor")) 0)
            (`self.K2_DestroyActor` (`self.Entity`))
            (else
              (`KismetArrayLibrary.Array_Add` (`self.Entities`) (`self.Entity`))))))
      (else
        (break))))
  (if (`self.PrintDebugMessages?`)
    (`KismetSystemLibrary.PrintString` (`KismetStringLibrary.Concat_StrStr` (`KismetSystemLibrary.GetDisplayName` self) " spawned " (`KismetStringLibrary.Conv_IntToString` (`KismetArrayLibrary.Array_Length` (`self.Entities`))) " entities.") true true (struct :`B` 1.0 :`A` 1.0)))
  (if _spawndata_behaviour_playonspawn_
    (`self.PlayBehaviour`)))

(event `PlayBehaviour`
  (bind (_spawndata_spawn_delaybeforespawnstart _spawndata_spawn_amountofentities _spawndata_behaviour_playonspawn_ _spawndata_behaviour_delaybetweeneachplay _spawndata_behaviour_randomizedelay_ _spawndata_behaviour_randomizefactor) (break `/Game/TPS_Game/Blueprints/System/S_IaSpawnData` (`self.SpawnData`)))
  (bind _entities (`self.Entities`))
  (bind _index (`self.For Loop With Delay` 0 (`KismetArrayLibrary.Array_Length` _entities) (`KismetMathLibrary.SelectFloat` (`KismetMathLibrary.RandomFloatInRange` (- _spawndata_behaviour_delaybetweeneachplay _spawndata_behaviour_randomizefactor) (+ _spawndata_behaviour_delaybetweeneachplay _spawndata_behaviour_randomizefactor)) _spawndata_behaviour_delaybetweeneachplay _spawndata_behaviour_randomizedelay_))
    (:`Loop Body`
      (bind _output (`|GetArrayItem` _entities _index))
      (`/Engine/EditorBlueprintResources/StandardMacros.IsValid` _output
        (:`Is Valid`
          (message `/Game/TPS_Game/Blueprints/System/BPI_IaControls.IA_PlayBehaviour` _output))))))

(fn `UserConstructionScript`
  (bind (_spawnareasize_x _spawnareasize_y) (`KismetMathLibrary.BreakVector2D` (`self.SpawnAreaSize`)))
  (`BoxComponent.SetBoxExtent` (`self.Spawn_Zone`) (`KismetMathLibrary.MakeVector` _spawnareasize_x _spawnareasize_y (.z (`.BoxExtent` (`KismetSystemLibrary.GetComponentBounds` (`self.Spawn_Zone`))))) true)
  (`SceneComponent.K2_AddLocalRotation` (`self.Spawn_Direction`) (`KismetMathLibrary.MakeRotator` 0.0 0.0 (`self.SpawnDirection`)) false false)
  (`SceneComponent.SetHiddenInGame` (`self.Spawn_Zone`) (not (`self.SpawnZoneVisibleInGame?`)) false)
  (`SceneComponent.SetHiddenInGame` (`self.Icon`) (not (`self.SpawnZoneVisibleInGame?`)) false))