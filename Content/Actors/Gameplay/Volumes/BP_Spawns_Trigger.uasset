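; BP_Spawns_Trigger is a box trigger volume that tells its controlled spawners to spawn when an actor of a listed class enters.
; Entry sends IASpawnMessage to each spawner, matching exact classes only, and records the overlapping actor.
; That actor's exit disables the trigger unless it is Reusable, and IAReset re-arms it and resets the spawners.
; The construction script sets the box size and in-game visibility of box and icon.
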(event `/Game/TPS_Game/Blueprints/System/BPI_IaControls.IA_Reset`
  (set `self.CanBeUsed?` true)
  (`|ExecutionSequence`
    (:`then_0`
      (for _array_element (`self.ControlledSpawners`)
        (`/Game/TPS_Game/Blueprints/Volumes/BP_Spawns_Spawner.IA_Reset` _array_element)))
    (:`then_1`
      (goto _label :!via `Break`))))

(event `self.InteractionArea.OnComponentBeginOverlap`
  (params (OverlappedComponent :type "PrimitiveComponent Object Reference") (OtherActor :type "Actor Object Reference") (OtherComp :type "PrimitiveComponent Object Reference") (OtherBodyIndex :type Integer) (bFromSweep :type Boolean) (SweepResult :type "HitResult Structure (by ref)"))
  (if (`self.CanBeUsed?`)
    (if (`KismetArrayLibrary.Array_Contains` (`self.OverlappingClasses`) (`GameplayStatics.GetObjectClass` OtherActor))
      (set `self.OverlappingActor` OtherActor)
      (for _array_element (`self.ControlledSpawners`) :!label _label
        (message `/Game/TPS_Game/Blueprints/System/BPI_IaControls.IA_Spawn` _array_element)))))

(event `self.InteractionArea.OnComponentEndOverlap`
  (params (OverlappedComponent :type "PrimitiveComponent Object Reference") (OtherActor :type "Actor Object Reference") (OtherComp :type "PrimitiveComponent Object Reference") (OtherBodyIndex :type Integer))
  (if (== OtherActor (`self.OverlappingActor`))
    (if (`self.Reusable?`)
      (set `self.CanBeUsed?` true)
      (else
        (set `self.CanBeUsed?` false)))))

(fn `UserConstructionScript`
  (`BoxComponent.SetBoxExtent` (`self.InteractionArea`) (`self.InteractionZone_Size`) true)
  (`SceneComponent.SetHiddenInGame` (`self.InteractionArea`) (not (`self.InteractionZone_VisibleInGame?`)) false)
  (`SceneComponent.SetHiddenInGame` (`self.Icon`) (not (`self.InteractionZone_VisibleInGame?`)) false))