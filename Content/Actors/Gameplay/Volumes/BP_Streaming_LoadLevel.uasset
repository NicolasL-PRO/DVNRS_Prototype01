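; Trigger volume that switches to a named level when an actor of one of the triggering classes enters its kill zone.
; The first valid overlap unpossesses the player, removes default pawn HUD widgets and destroys the pawn as cosmetic cleanup.
; In parallel, a delayed Open Level call performs a full level change, despite the Streaming name.
; The construction script sets the box's size and in-game visibility.
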(event `self.Kill_Zone.OnComponentBeginOverlap`
  (params (OverlappedComponent :type "PrimitiveComponent Object Reference") (OtherActor :type "Actor Object Reference") (OtherComp :type "PrimitiveComponent Object Reference") (OtherBodyIndex :type Integer) (bFromSweep :type Boolean) (SweepResult :type "HitResult Structure (by ref)"))
  (bind _returnvalue (`GameplayStatics.GetPlayerController` 0))
  (if (and (`KismetArrayLibrary.Array_Contains` (`self.TriggeringClasses`) (`GameplayStatics.GetObjectClass` OtherActor)) (!= (`self.NewLevelToLoadOnKill`) "None"))
    (`/Engine/EditorBlueprintResources/StandardMacros.DoOnce` false
      (:`Completed`
        ;[1 1 1] Deleting all Pawns from current level prior to loading the desired one (purely cosmetic)
        (`|ExecutionSequence`
          (:`then_0`
            (set `self.ControlledPawn` (`Controller.K2_GetPawn` _returnvalue))
            (`Controller.UnPossess` _returnvalue)
            (`KismetSystemLibrary.Delay` 0.25)
            (bind _foundwidgets (`WidgetBlueprintLibrary.GetAllWidgetsOfClass` "/Game/Ui/WBP_PlayerPawn_Default.WBP_PlayerPawn_Default_C"))
            (for _array_element _foundwidgets
              (`Widget.RemoveFromParent` _array_element))
            (`KismetSystemLibrary.Delay` 0.5)
            (`self.K2_DestroyActor` (`self.ControlledPawn`)))
          (:`then_1`
            (`KismetSystemLibrary.Delay` 1.0)
            (`KismetSystemLibrary.Delay` 1.0)
            (`GameplayStatics.OpenLevel` (`self.NewLevelToLoadOnKill`))))))))

(fn `UserConstructionScript`
  (bind (_killzone_areasize_x _killzone_areasize_y _killzone_areasize_z) (`KismetMathLibrary.BreakVector` (`self.KillZone_AreaSize`)))
  (`BoxComponent.SetBoxExtent` (`self.Kill_Zone`) (`KismetMathLibrary.MakeVector` _killzone_areasize_x _killzone_areasize_y _killzone_areasize_z) true)
  (`SceneComponent.SetHiddenInGame` (`self.Kill_Zone`) (not (`self.KillZone_VisibleInGame?`)) false)
  (`SceneComponent.SetHiddenInGame` (`self.Billboard`) (not (`self.KillZone_VisibleInGame?`)) false))