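; BP_INST_DoorA is an interactive door that toggles between open and closed when triggered.
; It infers its starting state from the DoorFrame yaw at BeginPlay, then plays the opening or closing sequence on each trigger.
; Door start and finish events update the open state and lock out retriggering during motion.
; It also tracks a NoOverlap flag, cleared on trigger and set when overlap ends.
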(event `self.ReceiveBeginPlay`
  (bind (_relativerotation_roll _relativerotation_pitch _relativerotation_yaw) (`KismetMathLibrary.BreakRotator` (`SceneComponent.RelativeRotation` (`self.Door_Frame`))))
  (bind (_relativerotation_roll_2 _relativerotation_pitch_2 _relativerotation_yaw_2) (`KismetMathLibrary.BreakRotator` (`SceneComponent.RelativeRotation` (`self.Door_Frame`))))
  (if (== _relativerotation_yaw 0.0)
    (set `self.DoorOpen?` false)
    (elif (== _relativerotation_yaw_2 -90.0)
      (set `self.DoorOpen?` true))))

(event `self.TriggerBehaviour`
  (set `self.NoOverlap` false)
  (if (`self.CanPlayAnimation?`)
    (if (`self.DoorOpen?`)
      (`ActorSequenceComponent.PlaySequence` (`self.Door_Closing`))
      (else
        (`ActorSequenceComponent.PlaySequence` (`self.Door_Opening`))))))

(event `DoorIsOpening`
  (set `self.CanPlayAnimation?` false))

(event `Door Opened`
  (set `self.CanPlayAnimation?` true)
  (set `self.DoorOpen?` true))

(event `DoorIsClosing`
  (set `self.CanPlayAnimation?` false))

(event `Door Closed`
  (set `self.CanPlayAnimation?` true)
  (set `self.DoorOpen?` false))

(event `self.OverlapEnded`
  (set `self.NoOverlap` true))

(fn `UserConstructionScript`
  (`parent.UserConstructionScript`)
  (set `self.CanPlayAnimation?` true))