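; Parent Blueprint for interactive objects, providing a proximity prompt and interaction entry points for characters.
; InteractionArea overlaps show a shop-near-player widget to player 0 and remove it on exit, then fire OverlapEnded.
; InteractMP and InteractMPServer store caller references and share a path to TriggerBehaviour; it and OverlapEnded are empty hooks.
; InteractionEnabled gates overlaps and interactions, and sets icon visibility in the construction script.
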(event `self.Interaction Area.OnComponentBeginOverlap`
  (params (OverlappedComponent :type "PrimitiveComponent Object Reference") (OtherActor :type "Actor Object Reference") (OtherComp :type "PrimitiveComponent Object Reference") (OtherBodyIndex :type Integer) (bFromSweep :type Boolean) (SweepResult :type "HitResult Structure (by ref)"))
  (bind _returnvalue (`GameplayStatics.GetPlayerController` 0))
  (if (`self.InteractionEnabled?`)
    (`/Engine/EditorBlueprintResources/StandardMacros.IsValid` OtherActor
      (:`Is Valid`
        (bind _asbp_character_base (cast `/Game/TPS_Game/Blueprints/System/BP_CharacterBase` OtherActor))
        (bind _owningplayercontroller (`/Game/TPS_Game/Blueprints/System/BP_CharacterBase.OwningPlayerController` _asbp_character_base)
          (:`then`
            (`/Engine/EditorBlueprintResources/StandardMacros.IsValid` _asbp_character_base
              (:`Is Valid`
                (bind _output_get (set `self.User` _owningplayercontroller))
                (if (== _output_get _returnvalue)
                  (bind _returnvalue_2 (`|CreateWidget` "/Game/TPS_Game/Blueprints/Bonus/Shop/W_ShopNearPlayer.W_ShopNearPlayer_C" _returnvalue))
                  (set `self.ShopInteractMessage` _returnvalue_2)
                  (bind _shopinteractmessage (`self.ShopInteractMessage`)
                    (:`then`
                      (`UserWidget.AddToViewport` _shopinteractmessage -1)
                      (`self.User`
                        (:`then`)
                        (:`else`)))
                    (:`else`))))))
          (:`else`))))))

(event `self.Interaction Area.OnComponentEndOverlap`
  (params (OverlappedComponent :type "PrimitiveComponent Object Reference") (OtherActor :type "Actor Object Reference") (OtherComp :type "PrimitiveComponent Object Reference") (OtherBodyIndex :type Integer))
  (if (`self.InteractionEnabled?`)
    (bind _asbp_character_base (cast `/Game/TPS_Game/Blueprints/System/BP_CharacterBase` OtherActor))
    (bind _shopinteractmessage (`self.ShopInteractMessage`)
      (:`then`
        (if (== (`Widget.GetOwningPlayer` _shopinteractmessage) (`/Game/TPS_Game/Blueprints/System/BP_CharacterBase.OwningPlayerController` _asbp_character_base))
          (bind _shopinteractmessage_2 (`self.ShopInteractMessage`)
            (:`then`
              (`Widget.RemoveFromParent` _shopinteractmessage_2)
              (set `self.ShopInteractMessage` null)
              (`self.OverlapEnded`))
            (:`else`))))
      (:`else`))))

(event `/Game/TPS_Game/Blueprints/System/BPI_Interact_MP.Interact_MP`
  (params (CharacterReference :type "/Game/TPS_Game/Blueprints/System/BP_CharacterBase Object Reference") (ControllerReference :type "/Game/TPS_Game/Blueprints/System/BP_PlayerController Object Reference"))
  (if (`self.InteractionEnabled?`)
    (set `self.Character Reference` CharacterReference)
    (set `self.Controller Reference` ControllerReference)
    (`/Engine/EditorBlueprintResources/ActorMacros.Switch Has Authority` :!label _label
      (:`Authority`
        _)
      (:`Remote`
        _))
    (`self.TriggerBehaviour`)))

(event `/Game/TPS_Game/Blueprints/System/BPI_Interact_MP_Server.Interact_MP_Server`
  (params (ControllerReference :type "/Game/TPS_Game/Blueprints/System/BP_PlayerController Object Reference"))
  (if (`self.InteractionEnabled?`)
    (set `self.Controller Reference` ControllerReference)
    (goto _label)))

(event `TriggerBehaviour`)

(event `OverlapEnded`)

(fn `UserConstructionScript`
  (`SceneComponent.SetVisibility` (`self.Interaction Icon`) (`self.InteractionEnabled?`) false))