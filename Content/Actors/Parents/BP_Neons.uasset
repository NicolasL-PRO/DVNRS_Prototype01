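; Parent neon Blueprint that pairs an emissive mesh with a rect light and an optional, quarter-strength point backlight.
; The construction script creates the dynamic material and applies color, intensity and radius, or blacks everything out when turned off.
; If enabled, flickering loops with random delays, speeds and one of three timeline curves, driving both lights and the material.
; A color-change event lerps only the lights to a new color by timeline.
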(event `self.ReceiveBeginPlay`
  (if (and (not (`self.TurnOff?`)) (`self.EnableFlickering?`))
    (`self.Flickering`)))

(event `ChangeLightColor_Event`
  (params (NewColor :type "LinearColor Structure"))
  (set `self.LightColor_New` NewColor)
  (`TimelineComponent.SetPlayRate` (`self.Animation_ColorSwap`) (`self.LightSwapSpeed`))
  (bind (_direction _alpha_value) (`Timeline|Animation_ColorSwap` :!via `PlayFromStart`)
    (:`Update`
      (bind _returnvalue (`KismetMathLibrary.LinearColorLerp` (`self.LightColor_Current`) (`self.LightColor_New`) _alpha_value))
      (`LightComponent.SetLightColor` (`self.Neon_PointLight`) _returnvalue true)
      (`LightComponent.SetLightColor` (`self.Neon_RectLight`) _returnvalue true))
    (:`Finished`
      (set `self.LightColor_Current` (`self.LightColor_New`)))))

(event `Flickering`
  (`KismetSystemLibrary.Delay` (`KismetMathLibrary.RandomFloatInRange` 1.0 5.0))
  (`TimelineComponent.SetPlayRate` (`self.Animation_Flickers`) (`KismetMathLibrary.RandomFloatInRange` 0.75 1.5))
  (set `self.Flicker_Selector` (`KismetMathLibrary.RandomIntegerInRange` 0 2))
  (bind (_direction _flicker01 _flicker02 _flicker03) (`Timeline|Animation_Flickers` :!via `PlayFromStart`)
    (:`Update`
      (bind _returnvalue (select `int` (`self.Flicker_Selector`) :`0` _flicker01 :`1` _flicker02 :`2` _flicker03))
      (`LightComponent.SetIntensity` (`self.Neon_PointLight`) (* (* (`self.Intensity`) 0.25) _returnvalue))
      (`LightComponent.SetIntensity` (`self.Neon_RectLight`) (* (`self.Intensity`) _returnvalue))
      (`MaterialInstanceDynamic.SetScalarParameterValue` (`self.MI_Neon`) "Emissive Strength" (* (`self.Emissive`) _returnvalue))
      (`MaterialInstanceDynamic.SetScalarParameterValue` (`self.MI_Neon`) "Color Intensity" _returnvalue))
    (:`Finished`
      (`self.Flickering`))))

(fn `UserConstructionScript`
  (bind _returnvalue (`KismetMathLibrary.SelectFloat` 0.0 (`self.Intensity`) (`self.TurnOff?`)))
  (bind _returnvalue_2 (`KismetMathLibrary.SelectColor` (struct) (`self.Color`) (`self.TurnOff?`)))
  (bind _returnvalue_3 (`PrimitiveComponent.CreateDynamicMaterialInstance` (`self.Neon_Mesh`) 1 "/Game/TPS_Game/Shaders/M_Scalar_Emissive.M_Scalar_Emissive" "None"))
  (set `self.MI_Neon` _returnvalue_3)
  ;[1 1 1] Lights Parameters
  (`MaterialInstanceDynamic.SetVectorParameterValue` (`self.MI_Neon`) "Color" (`KismetMathLibrary.SelectColor` (struct) (`self.Color`) (`self.TurnOff?`)))
  (`MaterialInstanceDynamic.SetScalarParameterValue` (`self.MI_Neon`) "Emissive Strength" (`KismetMathLibrary.SelectFloat` 0.0 (`self.Emissive`) (`self.TurnOff?`)))
  (`LightComponent.SetLightColor` (`self.Neon_PointLight`) _returnvalue_2 true)
  (`LightComponent.SetLightColor` (`self.Neon_RectLight`) _returnvalue_2 true)
  (`LightComponent.SetIntensity` (`self.Neon_PointLight`) (* _returnvalue 0.25))
  (`LightComponent.SetIntensity` (`self.Neon_RectLight`) _returnvalue)
  (`LocalLightComponent.SetAttenuationRadius` (`self.Neon_PointLight`) (* (`self.Radius`) 0.25))
  (`LocalLightComponent.SetAttenuationRadius` (`self.Neon_RectLight`) (`self.Radius`))
  (`SceneComponent.SetVisibility` (`self.Neon_PointLight`) (select `bool` (`self.UseBackLight?`) :`true` true) false)
  (set `self.LightColor_Current` (`self.Color`)))