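; BP_INST_DoorA is a scripted interactable door with an animated handle; the door swing itself is not implemented here.
; BehaviourPlay checks DoorOpen, printing "Close" if open, otherwise printing "Open" and playing the handle animation.
; A speed-adjustable timeline pitches the handle down and back by reversing itself after a short delay, tracking HandleAnimationPlaying.
; The construction script only calls the parent; material and initial door-rotation setup are disconnected.
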(event `self.Behaviour Play`
  (if (`self.DoorOpen?`)
    (`KismetSystemLibrary.PrintString` "Close")
    (else
      (`KismetSystemLibrary.PrintString` "Open")
      (`self.Play Door Handle Animation`))))

(event `Play Door Handle Animation`
  ; Door Handle Animation
  (`TimelineComponent.SetPlayRate` (`self.Door Handle Animation`) (`self.AnimationsSpeed`))
  (bind (_direction _alpha_value) (`Timeline|Door Handle Animation` :!label _label)
    (:`Update`
      (set `self.Handle_Animation_Playing?` true)
      (`SceneComponent.K2_SetRelativeRotation` (`self.DoorA_Handle`) (`KismetMathLibrary.MakeRotator` 0.0 (`KismetMathLibrary.Lerp` 0.0 45.0 _alpha_value)) false false))
    (:`Finished`
      (switch `ETimelineDirection` _direction
        (:`Forward`
          (`KismetSystemLibrary.Delay` 0.25)
          (goto _label :!via `Reverse`))
        (:`Backward`
          (set `self.Handle_Animation_Playing?` false))))))

(fn `UserConstructionScript`
  (`parent.UserConstructionScript`))