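; Base interactive actor, apparently meant to let pawns trigger a behaviour through an interface message, with empty event stubs for both.
; Construction picks a tagged box, capsule or sphere trigger, falling back to a default box, colours the arrow by interactivity and adds an "Interactive" tag.
; DoOnce gates with delayed resets are built to rate-limit triggering.
; The enabled, class, overlap and input checks feeding them are disconnected, as are UI updates.
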(event `self.ReceiveTick`
  (params (DeltaSeconds :type "Float (single-precision)")))

(event `/Game/Blueprints/BPI_Default.Pawn_ToInteractiveActor`
  (params (From :type "Actor Object Reference") (`Pawn Interaction Input Used?` :type "/Game/Blueprints/Tools/E_InteractionInput_State Enum" :default "NewEnumerator9") (`Pawn Current UI` :type "UserWidget Object Reference") (`Pawn Eyes Sights Data` :type "HitResult Structure")))

(event `Reset Behaviour`
  (`|ExecutionSequence`
    (:`then_0`
      (`/Engine/EditorBlueprintResources/StandardMacros.DoOnce` false :!via `Reset`
        (:`Completed`
          (`self.TriggerBehaviour_Event`)
          (`KismetSystemLibrary.PrintString` (`KismetStringLibrary.Concat_StrStr` (`KismetSystemLibrary.GetDisplayName` (`.HitActor` (`GameplayStatics.BreakHitResult` (stale `/Game/Blueprints/BPI_Default.Pawn_ToInteractiveActor` `Pawn Eyes Sights Data`)))) " has interacted with" (`KismetSystemLibrary.GetDisplayName` self) "; triggering behaviour.") :!label _label)
          (`KismetSystemLibrary.Delay` (`self.DelayBetweenTriggers`))
          (`self.Reset Behaviour`))))
    (:`then_1`
      (`/Engine/EditorBlueprintResources/StandardMacros.DoOnce` false :!via `Reset`
        (:`Completed`
          (`self.TriggerBehaviour_Event`)
          (goto _label))))))

(event `TriggerBehaviour_Event`)

(fn `IsOtherActorBelowDistanceWithSelf?`
  (params (OtherActor :type "Actor Object Reference") (Distance :type "Float (double-precision)"))
  (returns (ReturnValue :type Boolean))
  (return (<= (`self.GetDistanceTo` OtherActor) Distance)))

(fn `UserConstructionScript`
  (locals (Color_Interactive :type "Color Structure" :default (struct :`G` 255 :`A` 255)) (Color_Inactive :type "Color Structure" :default (struct :`R` 255 :`A` 255)))
  (bind _returnvalue (`self.GetComponentsByTag` "/Script/Engine.BoxComponent" "None"))
  (bind _returnvalue_2 (`self.GetComponentsByTag` "/Script/Engine.SphereComponent" "None"))
  (bind _returnvalue_3 (`self.GetComponentsByTag` "/Script/Engine.CapsuleComponent" "None"))
  (bind _returnvalue_4 (`self.GetComponentsByTag` "/Script/Engine.StaticMeshComponent" "None"))
  (`KismetArrayLibrary.Array_Clear` (`self.Tags`))
  ;[1 1 1] Display/Hide In Game
  (`SceneComponent.SetHiddenInGame` (`self.Arrow`) (not (`self.DisplayInGame?`)) false)
  (`SceneComponent.SetHiddenInGame` (`self.DefaultTriggerBox`) (not (`self.DisplayInGame?`)) false)
  ;[1 1 1] Box overlap setup
  (`SceneComponent.K2_SetRelativeLocation` (`self.DefaultTriggerBox`) (`self.DefaultTriggerBox_Position`) false false)
  (`BoxComponent.SetBoxExtent` (`self.DefaultTriggerBox`) (`self.DefaultTriggerBox_Size`) true)
  ;[1 1 1] Changes aspect and process flow on interactivity state
  (if (== (`self.InteractionEnabled?`) true)
    (set `ArrowComponent.ArrowColor` (`local.Color_Interactive`) (`self.Arrow`))
    (else
      (set `ArrowComponent.ArrowColor` (`local.Color_Inactive`) (`self.Arrow`))))
  ;[1 1 1] Interaction components selection process
  (if (!= (`KismetArrayLibrary.Array_Length` _returnvalue) 0)
    (set `self.Interaction_Trigger` (`|GetArrayItem` _returnvalue))
    (`SceneComponent.SetVisibility` (`self.DefaultTriggerBox`) false false :!label _label)
    (set `PrimitiveComponent.bGenerateOverlapEvents` false (`self.DefaultTriggerBox`))
    (if (!= (`KismetArrayLibrary.Array_Length` _returnvalue_4) 0) :!label _label_2
      (set `self.Interaction_Mesh` (`|GetArrayItem` _returnvalue_4)))
    ;;[1 1 1] Debug
    (`KismetSystemLibrary.PrintString` (`KismetSystemLibrary.GetDisplayName` (`self.Interaction_Trigger`)))
    (`KismetSystemLibrary.PrintString` (`KismetSystemLibrary.GetDisplayName` (`self.Interaction_Mesh`)))
    ;[1 1 1] Automatically adds a tag to the actor if not already present, and if it is set as interactive in Game Start (not during Runtime)
    (if (`self.Inactive?`)
      _
      (elif (not (`self.ActorHasTag` "Interactive"))
        (`KismetArrayLibrary.Array_Add` (`self.Tags`) "Interactive")))
    (elif (!= (`KismetArrayLibrary.Array_Length` _returnvalue_3) 0)
      (set `self.Interaction_Trigger` (`|GetArrayItem` _returnvalue_3))
      (goto _label)
      (elif (!= (`KismetArrayLibrary.Array_Length` _returnvalue_2) 0)
        (set `self.Interaction_Trigger` (`|GetArrayItem` _returnvalue_2))
        (else
          (set `self.Interaction_Trigger` (`self.DefaultTriggerBox`))
          (`KismetArrayLibrary.Array_Add` (`ActorComponent.ComponentTags` (`self.DefaultTriggerBox`)) "None")
          (set `PrimitiveComponent.bGenerateOverlapEvents` true (`self.DefaultTriggerBox`))
          (goto _label_2))))))