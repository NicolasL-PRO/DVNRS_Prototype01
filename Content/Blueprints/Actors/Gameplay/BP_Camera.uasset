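; Security camera actor that sweeps side to side and watches for targets through a vision sensing component.
; Timelines ping-pong the yaw continuously and dip the pitch after random delays, with a DoOnce gating each dip.
; Tick compares the sensing state with the previous one and fires an event on change, which currently only prints the results.
; The construction script derives sensing range, spotlight and vision cone mesh scale from distance and angle variables.
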(event `self.ReceiveBeginPlay`
  (`self.Camera_YawAnimation_Play` true))

(event `self.ReceiveTick`
  (params (DeltaSeconds :type "Float (single-precision)"))
  (bind (_vision_result_target _vision_result_sensingstate) (break `/Game/Blueprints/Tools/F_Sensing_Data` (`/Game/Blueprints/Components/SC_PawnSensing.Vision_Result` (`self.Camera_Sensing`))))
  (`|ExecutionSequence`
    (:`then_0`
      (`/Engine/EditorBlueprintResources/StandardMacros.DoOnce` false :!label _label
        (:`Completed`
          (`KismetSystemLibrary.RetriggerableDelay` (`KismetMathLibrary.RandomFloatInRange` 0.0 5.0))
          (`self.Camera_PitchAnimation_Play` false))))
    (:`then_1`
      (set `self.Vision_State_Current` _vision_result_sensingstate)
      (if (`|EnumInequality` (`self.Vision_State_Current`) (`self.Vision_State_Previous`))
        (`/Engine/EditorBlueprintResources/StandardMacros.DoOnce` false :!label _label_2
          (:`Completed`
            (set `self.Vision_State_Previous` (`self.Vision_State_Current`))
            (`self.Sense_Vision_Event` (`/Game/Blueprints/Components/SC_PawnSensing.Vision_Result` (`self.Camera_Sensing`)))
            (`self.Reset DoOnce Vision State Reading`)))))))

(event `Reset DoOnce Random LookDown`
  (goto _label :!via `Reset`))

(event `Reset DoOnce Vision State Reading`
  (goto _label_2 :!via `Reset`))

(event `Sense_Vision_Event`
  (params (`Vision Data` :type "/Game/Blueprints/Tools/F_Sensing_Data Structure"))
  (bind (_target _sensingstate _targetdistance _hitlocation _impactpoint) (break `/Game/Blueprints/Tools/F_Sensing_Data` `Vision Data`))
  (`KismetSystemLibrary.PrintString` (`KismetStringLibrary.Concat_StrStr` "*** VISION RESULTS ***" "TARGET: " (`KismetSystemLibrary.GetDisplayName` _target) " | " " STATE: " (`|GetEnumeratorNameAsString` _sensingstate) " | " "DISTANCE: " (`KismetStringLibrary.Conv_DoubleToString` _targetdistance) "LOCATION:  " (`KismetStringLibrary.Conv_VectorToString` _hitlocation) " | " "IMPACT: " (`KismetStringLibrary.Conv_VectorToString` _impactpoint))))

(event `Camera_YawAnimation_Play`
  (params (`Loop?` :type Boolean))
  (bind _camera (`self.Camera`))
  (bind (_relativerotation_roll _relativerotation_pitch) (`KismetMathLibrary.BreakRotator` (`SceneComponent.RelativeRotation` _camera)))
  ;[1 1 1] ANIMATIONS
  ;;[1 1 1] Camera Yaw Animation
  (`TimelineComponent.SetPlayRate` (`self.Camera_Rotation_Yaw`) 0.25)
  (if (not (`|EnumEquality` (`self.Camera_YawAnimation_Direction`) "Forward"))
    (bind (_direction _alpha) (`Timeline|Camera_Rotation_Yaw` :!label _label_3)
      (:`Update`
        (set `self.Camera_YawAnimation_Direction` _direction)
        (`SceneComponent.K2_SetRelativeRotation` _camera (`KismetMathLibrary.MakeRotator` _relativerotation_roll _relativerotation_pitch (`KismetMathLibrary.Lerp` -90.0 90.0 _alpha)) false false))
      (:`Finished`
        (if `Loop?`
          (`self.Camera_YawAnimation_Play` true))))
    (else
      (goto _label_3 :!via `Reverse`))))

(event `Camera_YawAnimationStop`
  ;[1 1 1] ANIMATIONS
  ;;[1 1 1] Camera Yaw Animation
  (goto _label_3 :!via `Stop`))

(event `Camera_PitchAnimation_Play`
  (params (`Loop?` :type Boolean))
  (bind _camera (`self.Camera`))
  (bind (_relativerotation_roll _relativerotation_pitch _relativerotation_yaw) (`KismetMathLibrary.BreakRotator` (`SceneComponent.RelativeRotation` _camera)))
  ;[1 1 1] ANIMATIONS
  ;;[1 1 1] Camera Pitch Animartion
  (`TimelineComponent.SetPlayRate` (`self.Camera_Rotation_Pitch`) 2.0)
  (if (not (`|EnumEquality` (`self.Camera_PitchAnimation_Direction`) "Forward"))
    (bind (_direction _alpha) (`Timeline|Camera_Rotation_Pitch` :!label _label_4)
      (:`Update`
        (set `self.Camera_PitchAnimation_Direction` _direction)
        (`SceneComponent.K2_SetRelativeRotation` _camera (`KismetMathLibrary.MakeRotator` _relativerotation_roll (`KismetMathLibrary.Lerp` 0.0 -22.5 _alpha) _relativerotation_yaw) false false))
      (:`Finished`
        (if (`|EnumEquality` (`self.Camera_PitchAnimation_Direction`) "Backward")
          (`self.Reset DoOnce Random LookDown`)
          (else
            (`self.Camera_PitchAnimation_Play` false)))))
    (else
      (goto _label_4 :!via `ReverseFromEnd`))))

(event `Camera_PitchAnimation_Stop`
  ;[1 1 1] ANIMATIONS
  ;;[1 1 1] Camera Pitch Animartion
  (goto _label_4 :!via `Stop`))

(fn `Reset DoOnce`)

(fn `UserConstructionScript`
  (bind _camera_sensing (`self.Camera_Sensing`))
  (bind _vision_range_max (`/Game/Blueprints/Components/SC_PawnSensing.Vision_Range_Max` (`self.Camera_Sensing`)))
  (bind _vision_angle (`/Game/Blueprints/Components/SC_PawnSensing.Vision_Angle` (`self.Camera_Sensing`)))
  (bind _returnvalue (/ (* (* _vision_range_max 2.0) (`KismetMathLibrary.DegTan` (`/Game/Blueprints/Components/SC_PawnSensing.Vision_Angle` (`self.Camera_Sensing`)))) 100.0))
  (bind _output_get (set `/Game/Blueprints/Components/SC_PawnSensing.Vision_Range_Max` (`self.Vision Distance`) _camera_sensing))
  (set `/Game/Blueprints/Components/SC_PawnSensing.Vision_Range_Min` (* _output_get 0.5) _camera_sensing)
  (set `/Game/Blueprints/Components/SC_PawnSensing.Vision_Angle` (`self.Vision Angle`) _camera_sensing)
  (`LocalLightComponent.SetAttenuationRadius` (`self.Camera_Light`) (`/Game/Blueprints/Components/SC_PawnSensing.Vision_Range_Max` (`self.Camera_Sensing`)))
  (`SpotLightComponent.SetOuterConeAngle` (`self.Camera_Light`) _vision_angle)
  (`SpotLightComponent.SetInnerConeAngle` (`self.Camera_Light`) (* _vision_angle 0.75))
  (`SceneComponent.SetWorldScale3D` (`self.Vision_Cone`) (`KismetMathLibrary.MakeVector` (/ _vision_range_max 100.0) _returnvalue _returnvalue)))