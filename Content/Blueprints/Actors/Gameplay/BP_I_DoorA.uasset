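; Interactable hinged door that opens and closes when triggered, notifying the game mode each time.
; TriggerBehaviour checks the last door timeline direction: opening first turns the handle and then swings the door, while closing reverses the door alone.
; Two timeline-driven macros lerp handle pitch and door yaw, with the handle springing back after its turn.
; ListenOrders blocks open or close orders while the door swings.
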(event `self.Trigger Behaviour`
  (message `/Game/Blueprints/BPI_Default.GameManager_Message` (`GameplayStatics.GetGameMode`) self)
  (if (`self.ListenOrders?`)
    (if (`|EnumEquality` (`self.Door_AnimationDirection`) "Backward")
      (`TimelineComponent.SetPlayRate` (`self.Handle_AnimationTimeline`) 2.0)
      (bind (_direction _alpha_value) (`Timeline|Handle_AnimationTimeline` :!label _label)
        (:`Update`
          (`SceneComponent.K2_SetRelativeRotation` (`self.Door_Handle`) (`KismetMathLibrary.MakeRotator` 0.0 (`KismetMathLibrary.Lerp` 0.0 67.5 _alpha_value)) false false))
        (:`Finished`
          (if (`|EnumEquality` _direction "Forward")
            (`|ExecutionSequence`
              (:`then_0`
                (`TimelineComponent.SetPlayRate` (`self.Door_AnimationTimeline`) 1.0)
                (bind (_direction_2 _alphavalue) (`Timeline|Door_AnimationTimeline` :!label _label_2)
                  (:`Update`
                    (`SceneComponent.K2_SetRelativeRotation` (`self.Door_Door`) (`KismetMathLibrary.MakeRotator` 0.0 0.0 (`KismetMathLibrary.Lerp` 0.0 90.0 _alphavalue)) false false)
                    (set `self.ListenOrders?` false))
                  (:`Finished`
                    (set `self.Door_AnimationDirection` _direction_2)
                    (set `self.ListenOrders?` true))))
              (:`then_1`
                (`TimelineComponent.SetPlayRate` (`self.Handle_AnimationTimeline`) 0.0)
                (goto _label :!via `Reverse`))))))
      (else
        (`TimelineComponent.SetPlayRate` (`self.Handle_AnimationTimeline`) 1.5)
        (goto _label_2 :!via `Reverse`)))))

(fn `UserConstructionScript`
  (`parent.UserConstructionScript`))