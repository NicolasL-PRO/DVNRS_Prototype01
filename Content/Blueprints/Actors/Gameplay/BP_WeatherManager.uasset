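; Weather manager actor that drives a day/night cycle by rotating the sun light and updating the sky sphere.
; The construction script validates and binds both actors, then sets the time scale and initial sun and sky light settings.
; Each tick converts elapsed seconds into a day fraction for the sun's pitch and the in-game clock.
; It sends that time and a dawn/dusk-based night flag to the game mode.
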(event `self.ReceiveBeginPlay`
  (set `self.ElapsedTime` (/ (* (`self.Get Time as Seconds` (`self.StartTime`)) (`self.SecondPerDay`)) 86400.0)))

(event `self.ReceiveTick`
  (params (DeltaSeconds :type "Float (single-precision)"))
  (bind _day_fraction (`self.GetFractionOfDay`))
  (bind (_f_time_days _f_time_hours _f_time_minutes) (break `/Game/Blueprints/Tools/F_Time` (make `/Game/Blueprints/Tools/F_Time` (`KismetMathLibrary.FTrunc` _day_fraction) (`KismetMathLibrary.FTrunc` (* (mod _day_fraction 1.0) 24.0)) (`KismetMathLibrary.FTrunc` (mod (* _day_fraction 1440.0) 60.0)))))
  (set `self.ElapsedTime` (+ (`self.ElapsedTime`) DeltaSeconds))
  (`SceneComponent.K2_SetRelativeRotation` (`Light.LightComponent` (`self.SunLight`)) (`KismetMathLibrary.MakeRotator` 0.0 (+ (* (`self.GetFractionOfDay`) 360.0) 90.0) 22.5) false false)
  (`/Engine/EngineSky/BP_Sky_Sphere.UpdateSunDirection` (`self.SkySphere`))
  (bind _output_get (set `self.CurrentTime` (make `/Game/Blueprints/Tools/F_Time` _f_time_days _f_time_hours _f_time_minutes)))
  (bind _output_get_2 (set `self.IsNight?` (or (< _f_time_hours (`self.DawnTime`)) (>= _f_time_hours (`self.DuskTime`)))))
  (message `/Game/Blueprints/BPI_Default.GameManager_Weather` (`GameplayStatics.GetGameMode`) self _output_get _output_get_2))

(fn `Get Time as Seconds`
  (params (`Time Structure` :type "/Game/Blueprints/Tools/F_Time Structure"))
  (returns (ReturnValue :type Integer))
  (bind (_days _hours _minutes) (break `/Game/Blueprints/Tools/F_Time` `Time Structure`))
  (return (+ (* _days 86400) (* _hours 3600) (* _minutes 60))))

(fn `GetFractionOfDay`
  (returns (`Day Fraction` :type "Float (double-precision)"))
  (return (/ (`self.ElapsedTime`) (`self.SecondPerDay`))))

(fn `UserConstructionScript`
  (bind _sunlight (`self.SunLight`))
  (bind _skysphere (`self.SkySphere`))
  ;[1 1 1] Checks actors dependencies validities, sets variables accordingly and returns console messages.
  (`/Engine/EditorBlueprintResources/StandardMacros.IsValid` _sunlight
    (:`Is Valid`
      (set `self.SunLightSourceValid?` true)
      (`KismetSystemLibrary.PrintString` (`KismetStringLibrary.Concat_StrStr` (`KismetSystemLibrary.GetDisplayName` _sunlight) "is correctly set as Sun Light Source.")))
    (:`Is Not Valid`
      (set `self.SunLightSourceValid?` false)
      (`KismetSystemLibrary.PrintString` "WARNING: no correct Sun Light Source set - system won't work properly. Please select or create a Directional Light.")))
  (`/Engine/EditorBlueprintResources/StandardMacros.IsValid` _skysphere
    (:`Is Valid`
      (set `self.SkySphereValid?` true)
      (`KismetSystemLibrary.PrintString` (`KismetStringLibrary.Concat_StrStr` (`KismetSystemLibrary.GetDisplayName` _skysphere) " is correctly set as Sky Sphere; binding  " (`KismetSystemLibrary.GetDisplayName` _sunlight) " to it."))
      (set `/Engine/EngineSky/BP_Sky_Sphere.Directional light actor` _sunlight _skysphere))
    (:`Is Not Valid`
      (set `self.SkySphereValid?` false)
      (`KismetSystemLibrary.PrintString` "WARNING: no correct Sky Sphere set - system won't work properly. Please select or create a BP_SkySphere.")))
  ;[1 1 1] Sets initial values for time scale (in-game time)
  (set `self.SecondPerDay` (* (`self.MinutesPerDay`) 60.0))
  (set `self.ElapsedTime` (/ (* (`self.Get Time as Seconds` (`self.StartTime`)) (`self.SecondPerDay`)) 86400.0))
  ;[1 1 1] Sets initial values for Sun (Directional Light)
  (`LightComponent.SetLightColor` (`Light.LightComponent` (`self.SunLight`)) (`self.SunLightColor`) true)
  (`LightComponent.SetIntensity` (`Light.LightComponent` (`self.SunLight`)) (`self.SunLightMaxIntensity`))
  ;[1 1 1] Sets initial values for Sky (Sky Light)
  (`SkyLightComponent.SetLightColor` (`self.SkyLight`) (`self.SkyLightColor`))
  (`SkyLightComponent.SetIntensity` (`self.SkyLight`) (`self.SkyLightMinIntensity`))
  (set `self.SkySphereValid?` (`KismetSystemLibrary.IsValid` (`self.SkySphere`)))
  (`/Engine/EngineSky/BP_Sky_Sphere.RefreshMaterial` (`self.SkySphere`)))