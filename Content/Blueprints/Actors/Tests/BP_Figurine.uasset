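; BP_Figurine is a test display actor with a spotlit figurine that can spin around its vertical axis.
; The construction script sets the spotlight's color, intensity and temperature from variables.
; While Rotate is set, Tick adds world yaw from ApplyConstantRotation.
; That helper's graph scales delta time by speed and direction, defaulting zero direction to one; its yaw-range check selects between equal speeds.
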(event `self.ReceiveBeginPlay`)

(event `self.ReceiveTick`
  (params (DeltaSeconds :type "Float (single-precision)"))
  (bind _rotationspeed (`self.RotationSpeed`))
  (bind _rotationdirection (`self.RotationDirection`))
  (bind (_returnvalue_roll _returnvalue_pitch _returnvalue_yaw) (`KismetMathLibrary.BreakRotator` (`SceneComponent.K2_GetComponentRotation` (`self.Figurine`))))
  (if (`self.Rotate?`)
    (`SceneComponent.K2_AddWorldRotation` (`self.Figurine`) (`KismetMathLibrary.MakeRotator` 0.0 0.0 (* (* DeltaSeconds (`KismetMathLibrary.SelectFloat` _rotationspeed (* _rotationspeed 1.0) (`KismetMathLibrary.InRange_FloatFloat` _returnvalue_yaw -90.0 0.0))) (`KismetMathLibrary.SelectInt` (`self.RotationDirection`) 1 (or (> _rotationdirection 0) (< _rotationdirection 0))))) false false)))

(fn `UserConstructionScript`
  (`LightComponent.SetLightColor` (`self.SpotLight`) (`self.Light Color`) true)
  (`LightComponent.SetIntensity` (`self.SpotLight`) (`self.Light Intensity`))
  (`LightComponent.SetTemperature` (`self.SpotLight`) (`self.Light Temparature`)))