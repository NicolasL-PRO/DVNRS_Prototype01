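; Actor component that acts as a pawn's "eyes" for interacting with objects in the world.
; Every tick it runs a debug-drawable Visibility line trace over the sight range, chosen by camera type.
; First person traces along the current camera; third person traces from an eye socket to a point ahead of the capsule.
; Hit actors implementing BPI_Default receive PawnInteractionMessage with the owner, interaction input state and hit data.
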(event `self.ReceiveTick`
  (params (DeltaSeconds :type "Float (single-precision)"))
  (bind _pawncamera_current (`self.PawnCamera_Current`))
  (bind _pawn_capsulecollision (`self.Pawn_CapsuleCollision`))
  (bind (_location_start _location_end) (`/Game/Blueprints/Tools/BPL_MyFunctions.Compute Forward Location From Scene Components` _pawncamera_current _pawncamera_current (`self.Pawn_EyeSights_Range`)))
  (switch `/Game/Blueprints/Tools/E_Camera_ViewType` (`self.PawnCamera_CurrentType`)
    (:`NewEnumerator0`
      ;[1 1 1] Character "Eyes" and sight distance (use for interactions) - casted from pawn camera
      (bind _outhit (`KismetSystemLibrary.LineTraceSingle` :`Start` _location_start :`End` _location_end :`TraceChannel` "TraceTypeQuery1" :`DrawDebugType` (`self.Draw Debug Type`) :`TraceColor` (struct :`R` 0.413513 :`G` 0.446824 :`B` 1.0 :`A` 1.0) :`TraceHitColor` (struct :`R` 0.94902 :`G` 1.0 :`A` 1.0)))
      (bind _output_get (set `self.Pawn_EyesSights_CameraData` _outhit))
      (if (`KismetSystemLibrary.DoesImplementInterface` (`.HitActor` (`GameplayStatics.BreakHitResult` _output_get)) "/Game/Blueprints/BPI_Default.BPI_Default_C")
        (switch `/Game/Blueprints/Tools/E_Camera_ViewType` (`self.PawnCamera_CurrentType`)
          (:`NewEnumerator0`
            (message `/Game/Blueprints/BPI_Default.Pawn_Interaction` (`.HitActor` (`GameplayStatics.BreakHitResult` _output_get)) (`self.GetOwner`) (`self.Pawn_Interaction_InputUsed?`) (`self.Pawn_EyesSights_CameraData`))))))
    (:`NewEnumerator1`
      ;[1 1 1] Character "Eyes" and sight distance (use for interactions) - casted from pawn itself
      (bind _outhit_2 (`KismetSystemLibrary.LineTraceSingle` :`Start` (`SceneComponent.GetSocketLocation` (`self.Pawns_EyesSights_SocketOwner`) (`self.Pawns_EyesSights_SocketName`)) :`End` (`.Location End` (`/Game/Blueprints/Tools/BPL_MyFunctions.Compute Forward Location From Scene Components` _pawn_capsulecollision _pawn_capsulecollision (`self.Pawn_EyeSights_Range`))) :`TraceChannel` "TraceTypeQuery1" :`DrawDebugType` (`self.Draw Debug Type`) :`TraceColor` (struct :`R` 0.384455 :`G` 1.0 :`B` 0.370675 :`A` 1.0) :`TraceHitColor` (struct :`R` 0.887923 :`G` 1.0 :`A` 1.0)))
      (bind _output_get_2 (set `self.Pawn_EyesSights_CameraData` _outhit_2))
      (if (`KismetSystemLibrary.DoesImplementInterface` (`.HitActor` (`GameplayStatics.BreakHitResult` _output_get_2)) "/Game/Blueprints/BPI_Default.BPI_Default_C")
        (switch `/Game/Blueprints/Tools/E_Camera_ViewType` (`self.PawnCamera_CurrentType`)
          (:`NewEnumerator1`
            (message `/Game/Blueprints/BPI_Default.Pawn_Interaction` (`.HitActor` (`GameplayStatics.BreakHitResult` _output_get_2)) (`self.GetOwner`) (`self.Pawn_Interaction_InputUsed?`) (`self.Pawn_EyesSights_CameraData`))))))))