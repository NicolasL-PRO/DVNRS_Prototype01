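; Pawn sensing scene component that detects actors of target classes by sight; hearing is an empty stub.
; Looping timers for both senses share HearingInterval, and each vision tick stores Vision's result.
; Vision line-traces on Camera channel to target actors, tests cone angle and two ranges, and returns a tiered result from the first actor evaluated.
; Optional debug drawing shows both range cones and traces.
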(event `self.ReceiveBeginPlay`
  (`self.Begin Sensing`))

(event `Begin Sensing`
  ;[1 1 1] Begin Sensing procedure on specified interval
  (bind _returnvalue (`KismetSystemLibrary.K2_SetTimerDelegate` (delegate `Sensing Vision`) (`self.Hearing_Interval`) true))
  (set `self.Vision_Timer_Reference` _returnvalue)
  (bind _returnvalue_2 (`KismetSystemLibrary.K2_SetTimerDelegate` (delegate `Sensing Hearing`) (`self.Hearing_Interval`) true))
  (set `self.Hearing_Timer_Reference` _returnvalue_2))

(event `Sensing Vision`
  ;[1 1 1] Vision Function and component returns
  (bind _vision_result (`self.Vision`))
  (set `self.Vision Result` _vision_result))

(event `Sensing Hearing`)

(fn `Vision`
  (returns (Vision_Result :type "/Game/Blueprints/Tools/F_Sensing_Data Structure"))
  (locals (Vision_Raycast_HitResult_Current :type "HitResult Structure") (Vision_CurrentSeen_Actor :type "Actor Object Reference") (Vision_Raycast_DrawType :type "EDrawDebugTrace Enum") (Vision_Result_Local :type "/Game/Blueprints/Tools/F_Sensing_Data Structure"))
  (bind _vision_angle (`self.Vision_Angle`))
  (bind _vision_angle_2 (`self.Vision_Angle`))
  (bind (_vision_raycast_hitresult_current_bblockinghit _vision_raycast_hitresult_current_binitialoverlap _vision_raycast_hitresult_current_time _vision_raycast_hitresult_current_distance _vision_raycast_hitresult_current_location _vision_raycast_hitresult_current_impactpoint) (`GameplayStatics.BreakHitResult` (`local.Vision_Raycast_HitResult_Current`)))
  (bind _vision_currentseen_actor (`local.Vision_CurrentSeen_Actor`))
  ;[1 1 1] Script parameters
  (if (`self.Vision_ShowCone?`)
    (`KismetSystemLibrary.DrawDebugConeInDegrees` (`self.K2_GetComponentLocation`) (`self.GetForwardVector`) (`self.Vision_Range_Max`) _vision_angle _vision_angle 16 (struct :`R` 1.0 :`G` 0.743591 :`A` 1.0) (`self.Hearing_Interval`) 1.0)
    (`KismetSystemLibrary.DrawDebugConeInDegrees` (`self.K2_GetComponentLocation`) (`self.GetForwardVector`) (`self.Vision_Range_Min`) _vision_angle_2 _vision_angle_2 16 (struct :`R` 1.0 :`G` 0.047707 :`A` 1.0) (`self.Hearing_Interval`) 1.5))
  (for _array_element (`self.Sensing_Targets`)
    (bind _outactors (`GameplayStatics.GetAllActorsOfClass` _array_element))
    (for _array_element_2 _outactors
      (set `local.Vision_CurrentSeen_Actor` _array_element_2)
      ;[1 1 1] Raycasts to objects from defined classes
      (if (`self.Vision_ShowCone?`)
        (set `local.Vision_Raycast_DrawType` "ForOneFrame")
        (else
          (set `local.Vision_Raycast_DrawType` "None")))
      (bind (_outhit _returnvalue) (`KismetSystemLibrary.LineTraceSingle` (`self.K2_GetComponentLocation`) (`Actor.K2_GetActorLocation` (`local.Vision_CurrentSeen_Actor`)) "TraceTypeQuery2" false (`|MakeArray` (`self.GetOwner`)) (`local.Vision_Raycast_DrawType`)))
      ;[1 1 1] Hit Result intial conditions
      (if (and (`self.Vision_Active?`) _returnvalue)
        (bind _output_get (set `local.Vision_Raycast_HitResult_Current` _outhit))
        (if (== (`local.Vision_CurrentSeen_Actor`) (`.HitActor` (`GameplayStatics.BreakHitResult` _output_get)))
          ;[1 1 1] Sense scenarios on Hit Result intial conditions matched
          ;;[1 1 1] Within Vision Cone Angle Test
          (if (<= (`KismetMathLibrary.DegAcos` (`KismetMathLibrary.Dot_VectorVector` (`self.GetForwardVector` self) (`KismetMathLibrary.GetDirectionUnitVector` (`self.K2_GetComponentLocation` self) (`Actor.K2_GetActorLocation` (`local.Vision_CurrentSeen_Actor`))))) (`self.Vision_Angle`))
            ;;[1 1 1] In Sights Tests
            (if (<= (`.Distance` (`GameplayStatics.BreakHitResult` _output_get)) (`self.Vision_Range_Max`))
              (if (<= (`.Distance` (`GameplayStatics.BreakHitResult` _output_get)) (`self.Vision_Range_Min`))
                ;[1 1 1] Results and function returns
                (set `local.Vision_Result_Local` (make `/Game/Blueprints/Tools/F_Sensing_Data` _vision_currentseen_actor "NewEnumerator2" _vision_raycast_hitresult_current_distance _vision_raycast_hitresult_current_location _vision_raycast_hitresult_current_impactpoint))
                (else
                  (set `local.Vision_Result_Local` (make `/Game/Blueprints/Tools/F_Sensing_Data` _vision_currentseen_actor "NewEnumerator1" _vision_raycast_hitresult_current_distance _vision_raycast_hitresult_current_location _vision_raycast_hitresult_current_impactpoint))))
              (else
                (set `local.Vision_Result_Local` (make `/Game/Blueprints/Tools/F_Sensing_Data` null) :!label _label)))
            (else
              (goto _label)))
          (else
            (goto _label)))
        (else
          (goto _label)))
      (return (`local.Vision_Result_Local`)))))