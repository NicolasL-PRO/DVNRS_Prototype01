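; Default game mode that spawns the player pawn, assigns its first-person UI and relays in-game time to that UI.
; On BeginPlay it spawns the pawn at the first PlayerStart found and creates the widget.
; After a timed camera blend, it messages the pawn with controller, start and UI, then possesses it.
; Weather manager time updates are converted to display text and sent to the widget's log text.
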(event `self.ReceiveBeginPlay`
  ;[1 1 1] Events Begin Play
  (`|ExecutionSequence`
    (:`then_0`
      ;[1 1 1] Spawn Default Pawn at PlayerStart location, message it to possess and assign specified UI
      (bind _outactors (`GameplayStatics.GetAllActorsOfClass` "/Script/Engine.PlayerStart"))
      (bind _output_get (set `self.PlayerStart_Current` (`|GetArrayItem` _outactors)))
      (bind _returnvalue (`|SpawnActorFromClass` (`self.Player_PawnClass`) (`KismetMathLibrary.MakeTransform` (`self.K2_GetActorLocation` _output_get) (`self.K2_GetActorRotation` _output_get)) "AdjustIfPossibleButAlwaysSpawn" "MultiplyWithRoot" null null))
      (bind _instigator (`Actor.Instigator` _returnvalue))
      (`Pawn.SpawnDefaultController` _instigator)
      (bind _output_get_2 (set `self.PlayerPawn_Current` _instigator))
      (`KismetSystemLibrary.PrintString` (`KismetSystemLibrary.GetDisplayName` _output_get_2))
      (bind _returnvalue_2 (`|CreateWidget` "/Game/Blueprints/UI/WBP_FirstPerson_Default.WBP_FirstPerson_Default_C" (`GameplayStatics.GetPlayerController` 0)))
      (set `self.PlayerUI_Current` _returnvalue_2)
      (`PlayerController.SetViewTargetWithBlend` (`GameplayStatics.GetPlayerController` 0) (`self.PlayerPawn_Current`) (`self.Pawn_Possession_Camera_BlendTime`) "VTBlend_EaseOut" 1.0 false)
      (`KismetSystemLibrary.Delay` (`self.Pawn_Possession_Camera_BlendTime`))
      (message `/Game/Blueprints/BPI_Default.Pawn_Possess` (`self.PlayerPawn_Current`) (`GameplayStatics.GetPlayerController` 0) (`self.PlayerStart_Current`) (`self.PlayerUI_Current`))
      (`Controller.Possess` (`GameplayStatics.GetPlayerController` 0) (`self.PlayerPawn_Current`)))))

(event `/Game/Blueprints/BPI_Default.WeatherManager_UpdateTime`
  (params (From :type "Actor Object Reference") (` CurrentTime` :type "/Game/Blueprints/Tools/F_Time Structure") (Nighttime :type Boolean))
  ;[1 1 1] Reception of in-game time and process it to UI compliant format
  (bind _output_get (set `self.Time_UIDisplay` (`KismetTextLibrary.Conv_StringToText` (`KismetStringLibrary.Concat_StrStr` (`KismetStringLibrary.Concat_StrStr` (`KismetMathLibrary.SelectString` "0" "" (< ` CurrentTime_Hours_6_8EFE86564BB6AAFC67A3AF9A346DF96A` 10)) (`KismetStringLibrary.Conv_IntToString` ` CurrentTime_Hours_6_8EFE86564BB6AAFC67A3AF9A346DF96A`)) " : " (`KismetStringLibrary.Conv_IntToString` ` CurrentTime_Minutes_7_16DCD81E4F394CB0DBAD34A179113124`)))))
  (`/Game/Blueprints/BPI_Default.UI_SetLogText` (`self.PlayerUI_Current`) _output_get))

(fn `UserConstructionScript`)