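; Blueprint function library of general helpers for distance checks, forward-point math, component lookup, debug printing and interaction setup.
; The component lookup prefers a tagged match, otherwise returns the first of that class with Match false.
; Debug messages print under a header naming the calling world context object.
; An interaction setter copies pawn camera, eye-sight, capsule, input and debug-draw values onto an interact component, warning if it is invalid.
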(fn `Actors Are Below Distance?`
  (params (`Actor 1` :type "Actor Object Reference") (`Actor 2` :type "Actor Object Reference") (Distance :type "Float (double-precision)"))
  (returns (`Below?` :type Boolean))
  (return (<= (`Actor.GetDistanceTo` `Actor 1` `Actor 2`) Distance)))

(fn `Compute Forward Location From Scene Components`
  (params (`Location Source Component` :type "SceneComponent Object Reference") (`Forward Source Component` :type "SceneComponent Object Reference") (Distance :type "Float (double-precision)"))
  (returns (`Location Start` :type "Vector Structure") (`Location End` :type "Vector Structure"))
  (bind _returnvalue (`SceneComponent.K2_GetComponentLocation` `Location Source Component`))
  (return _returnvalue (+ _returnvalue (* (`SceneComponent.GetForwardVector` `Forward Source Component`) Distance))))

(fn `Debug Custom Message`
  (params (Text :type String) (PrintToScreen :type Boolean) (PrintToLog :type Boolean) (TextColor :type "LinearColor Structure") (Duration :type "Float (double-precision)"))
  (`KismetSystemLibrary.PrintString` null (`KismetStringLibrary.Concat_StrStr` ">>> MESSAGE FROM *" (`KismetSystemLibrary.GetDisplayName` (`local.__WorldContext`)) "*: ") PrintToScreen PrintToLog (struct :`R` 1.0 :`G` 0.990373 :`B` 0.933301 :`A` 1.0) Duration)
  (`KismetSystemLibrary.PrintString` null Text PrintToScreen PrintToLog TextColor)
  (return))

(fn `Get First Component of Class with Tag`
  (params (Target :type "Actor Object Reference") (Class :type "PrimitiveComponent Class Reference") (Tag :type Name))
  (returns (Match :type Boolean) (Component :type "PrimitiveComponent Object Reference"))
  (locals (`Is_There_A_Match?` :type Boolean) (Retrieved_Component :type "PrimitiveComponent Object Reference"))
  (if (!= (`KismetArrayLibrary.Array_Length` (`Actor.K2_GetComponentsByClass` Target Class)) 0)
    (if (!= (`KismetArrayLibrary.Array_Length` (`Actor.GetComponentsByTag` Target Class Tag)) 0)
      (set `local.Retrieved_Component` (`|GetArrayItem` (`Actor.GetComponentsByTag` Target Class Tag)))
      (set `local.Is_There_A_Match?` true)
      (else
        (set `local.Retrieved_Component` (`|GetArrayItem` (`Actor.K2_GetComponentsByClass` Target Class)))
        (set `local.Is_There_A_Match?` false :!label _label)))
    (else
      (set `local.Retrieved_Component` null)
      (goto _label)))
  (return (`local.Is_There_A_Match?`) (`local.Retrieved_Component`)))

(fn `Set Interact Component Parameters`
  (params (Component :type "/Game/Blueprints/Components/AC_Interact Object Reference") (PawnCamera_Current :type "CameraComponent Object Reference") (PawnCamera_CurrentType :type "/Game/Blueprints/Tools/E_Camera_ViewType Enum" :default "NewEnumerator0") (Pawn_EyeSights_Range :type "Float (double-precision)") (Pawn_CapsuleCollision :type "CapsuleComponent Object Reference") (Pawns_EyesSights_SocketOwner :type "SceneComponent Object Reference") (Pawns_EyesSights_SocketName :type Name) (`Pawn_Interaction_InputUsed?` :type "/Game/Blueprints/Tools/E_InteractionInput_State Enum" :default "NewEnumerator9") (`Draw Debug Type` :type "EDrawDebugTrace Enum" :default "None"))
  (`/Engine/EditorBlueprintResources/StandardMacros.IsValid` Component
    (:`Is Valid`
      (set `/Game/Blueprints/Components/AC_Interact.PawnCamera_Current` PawnCamera_Current Component)
      (set `/Game/Blueprints/Components/AC_Interact.PawnCamera_CurrentType` PawnCamera_CurrentType Component)
      (set `/Game/Blueprints/Components/AC_Interact.Pawn_EyesSights_Range` Pawn_EyeSights_Range Component)
      (set `/Game/Blueprints/Components/AC_Interact.Pawn_CapsuleCollision` Pawn_CapsuleCollision Component)
      (set `/Game/Blueprints/Components/AC_Interact.Pawns_EyesSights_SocketOwner` Pawns_EyesSights_SocketOwner Component)
      (set `/Game/Blueprints/Components/AC_Interact.Pawns_EyesSights_SocketName` Pawns_EyesSights_SocketName Component)
      (set `/Game/Blueprints/Components/AC_Interact.Pawn_Interaction_InputState` `Pawn_Interaction_InputUsed?` Component)
      (set `/Game/Blueprints/Components/AC_Interact.Draw Debug Type` `Draw Debug Type` Component))
    (:`Is Not Valid`
      (`KismetSystemLibrary.PrintString` null "*** WARNING: Interaction Component not found!" true true (struct :`R` 1.0 :`A` 1.0))))
  (return))