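; Pawn component that detects the interactive actor in the pawn's line of sight and notifies it.
; A gate opened on BeginPlay runs a Visibility line trace every Tick, from the camera in first person or a socket along capsule forward in third person.
; Hit actors implementing BPI_Default receive PawnToInteractiveActorMessage with the owner, input state, current UI and hit data, alongside a "Hello" debug print.
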(event `self.ReceiveBeginPlay`
  (`self.Fire Tick`))

(event `self.ReceiveTick`
  (params (DeltaSeconds :type "Float (single-precision)"))
  (bind _pawns_eyessights_socketowner (`self.Pawns_EyesSights_SocketOwner`))
  (bind _pawncamera_current (`self.PawnCamera_Current`))
  (bind _pawncamera_current_2 (`self.PawnCamera_Current`))
  (`/Engine/EditorBlueprintResources/StandardMacros.Gate` true :!label _label
    (:`Exit`
      ;[1 1 1] Draws an line to determine the interacted actor (relative to camera type) and sends it the interaction message if the interaction interface has been detected on it.
      (switch `/Game/Blueprints/Tools/E_Camera_ViewType` (`self.PawnCamera_CurrentType`)
        (:`NewEnumerator0`
          (set `self.Pawn_EyesSights_Start` (`/Game/Blueprints/Tools/BPL_MyFunctions.Compute Forward Location From Scene Components` _pawncamera_current _pawncamera_current (`self.Pawn_EyesSights_Range`)))
          (set `self.Pawn_EyesSights_End` (`.Location End` (`/Game/Blueprints/Tools/BPL_MyFunctions.Compute Forward Location From Scene Components` _pawncamera_current_2 _pawncamera_current_2 (`self.Pawn_EyesSights_Range`)))))
        (:`NewEnumerator1`
          (set `self.Pawn_EyesSights_Start` (`SceneComponent.GetSocketLocation` _pawns_eyessights_socketowner (`self.Pawns_EyesSights_SocketName`)))
          (set `self.Pawn_EyesSights_End` (`.Location End` (`/Game/Blueprints/Tools/BPL_MyFunctions.Compute Forward Location From Scene Components` _pawns_eyessights_socketowner (`self.Pawn_CapsuleCollision`) (`self.Pawn_EyesSights_Range`))))))
      (bind _outhit (`KismetSystemLibrary.LineTraceSingle` :`Start` (`self.Pawn_EyesSights_Start`) :`End` (`self.Pawn_EyesSights_End`) :`TraceChannel` "TraceTypeQuery1" :`DrawDebugType` (`self.Draw Debug Type`) :`TraceColor` (struct :`R` 0.413513 :`G` 0.446824 :`B` 1.0 :`A` 1.0) :`TraceHitColor` (struct :`R` 0.94902 :`G` 1.0 :`A` 1.0)))
      (bind _output_get (set `self.Pawn_EyesSights_CameraData` _outhit))
      (if (not (== (`.HitActor` (`GameplayStatics.BreakHitResult` _output_get)) null))
        (if (`KismetSystemLibrary.DoesImplementInterface` (`.HitActor` (`GameplayStatics.BreakHitResult` _output_get)) "/Game/Blueprints/BPI_Default.BPI_Default_C")
          (`KismetSystemLibrary.PrintString` "Hello")
          (message `/Game/Blueprints/BPI_Default.Pawn_ToInteractiveActor` (`.HitActor` (`GameplayStatics.BreakHitResult` _output_get)) (`self.GetOwner`) (`self.Pawn_Interaction_InputState`) (`self.Pawn_CurrentUI`) (`self.Pawn_EyesSights_CameraData`)))))))

(event `Fire Tick`
  (goto _label :!via `Open`))

(fn `Pawn_ToInteractiveActor`
  (params (From :type "Actor Object Reference") (`Pawn Interaction Input Used?` :type "/Game/Blueprints/Tools/E_InteractionInput_State Enum" :default "NewEnumerator9") (`Pawn Current UI` :type "UserWidget Object Reference") (`Pawn Eyes Sights Data` :type "HitResult Structure")))