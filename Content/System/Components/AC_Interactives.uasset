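; Actor component that detects interactive actors its owner overlaps, faces or looks at, and notifies them.
; Each Tick checks overlapping components and runs separate facing and looking sphere traces, filtering hits by class and component tag into three booleans.
; DoOnce-based macros turn boolean changes into one-shot Begin/End interface messages, clearing the actor reference after a tiny delay on End.
; Optional debug text prints all three states and targets.
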(event `self.ReceiveTick`
  (params (DeltaSeconds :type "Float (single-precision)"))
  (bind _facing_locationvector (`self.Facing_LocationVector`))
  (bind _looking_locationvector (`self.Looking_LocationVector`))
  (`|ExecutionSequence`
    (:`then_0`
      ; Overlapping Interactive Actor Test
      (bind _output_get (set `self.Overlapping_Components` (`Actor.GetOverlappingComponents` (`self.GetOwner` self))))
      (if (not (== (`KismetArrayLibrary.Array_Length` _output_get) 0))
        (for _array_element _output_get
          (bind _output_get_2 (set `self.Overlapping_Actor` (`self.GetOwner` _array_element)))
          (if (and (`KismetMathLibrary.ClassIsChildOf` (`GameplayStatics.GetObjectClass` _output_get_2) (`self.InteractiveActorsClass`)) (`self.ComponentHasTag` _array_element (`self.InteractiveComponentTag_Overlap`)))
            (set `self.Overlapping_InteractiveActor?` true)
            (break)))
        (else
          (set `self.Overlapping_InteractiveActor?` false))))
    (:`then_1`
      ; Facing Interactive Actor Test
      (bind _outhit (`KismetSystemLibrary.SphereTraceSingle` :`Start` _facing_locationvector :`End` (+ _facing_locationvector (* (`self.Facing_ForwardVector`) (`self.TraceDistance`))) :`Radius` (`self.Facing_TraceRadius`) :`TraceChannel` "TraceTypeQuery3" :`DrawDebugType` (`self.Facing_DrawDebugType`)))
      (if (`KismetSystemLibrary.IsValid` (`.HitActor` (`GameplayStatics.BreakHitResult` _outhit)))
        (bind _output_get_3 (set `self.Facing_Actor` (`.HitActor` (`GameplayStatics.BreakHitResult` _outhit))))
        (if (and (`KismetMathLibrary.ClassIsChildOf` (`GameplayStatics.GetObjectClass` _output_get_3) "/Game/Actors/+ParentActors/BP_Interactives.BP_Interactives_C") (`self.ComponentHasTag` (`.HitComponent` (`GameplayStatics.BreakHitResult` _outhit)) (`self.InteractiveComponentTag_FacingLooking`)))
          (set `self.Facing_InteractiveActor?` true)
          (else
            (set `self.Facing_InteractiveActor?` false :!label _label)))
        (else
          (goto _label))))
    (:`then_2`
      ; Looking at Interactive Actor Tests
      (bind _outhit_2 (`KismetSystemLibrary.SphereTraceSingle` :`Start` _looking_locationvector :`End` (+ _looking_locationvector (* (`self.Looking_ForwardVector`) (`self.TraceDistance`))) :`Radius` (`self.Looking_TraceRadius`) :`TraceChannel` "TraceTypeQuery3" :`DrawDebugType` (`self.Looking_DrawDebugType`)))
      (if (`KismetSystemLibrary.IsValid` (`.HitActor` (`GameplayStatics.BreakHitResult` _outhit_2)))
        (bind _output_get_4 (set `self.Looking_Actor` (`.HitActor` (`GameplayStatics.BreakHitResult` _outhit_2))))
        (if (and (`KismetMathLibrary.ClassIsChildOf` (`GameplayStatics.GetObjectClass` _output_get_4) "/Game/Actors/+ParentActors/BP_Interactives.BP_Interactives_C") (`self.ComponentHasTag` (`.HitComponent` (`GameplayStatics.BreakHitResult` _outhit_2)) (`self.InteractiveComponentTag_FacingLooking`)))
          (set `self.Looking_InteractiveActor?` true)
          (else
            (set `self.Looking_InteractiveActor?` false :!label _label_2)))
        (else
          (goto _label_2))))
    (:`then_3`
      ; If all Tests are True (with a second check to prevent errors with nearby Interactive Actors), send Implemented Interface Message (only once per Boolean change)
      (if (`self.DebugTexts?`)
        (`KismetSystemLibrary.PrintString` (`KismetStringLibrary.Concat_StrStr` (`KismetStringLibrary.Concat_StrStr` "OVERLAPPING: " (`KismetStringLibrary.Conv_BoolToString` (`self.Overlapping_InteractiveActor?`)) " | " (`KismetSystemLibrary.GetDisplayName` (`self.Overlapping_Actor`)) " \n") (`KismetStringLibrary.Concat_StrStr` "FACING: " (`KismetStringLibrary.Conv_BoolToString` (`self.Facing_InteractiveActor?`)) " | " (`KismetSystemLibrary.GetDisplayName` (`self.Facing_Actor`)) " \n") (`KismetStringLibrary.Concat_StrStr` "LOOKING: " (`KismetStringLibrary.Conv_BoolToString` (`self.Looking_InteractiveActor?`)) " | " (`KismetSystemLibrary.GetDisplayName` (`self.Looking_Actor`)) " \n"))))
      (`|ExecutionSequence`
        (:`then_0`
          (if (`self.Overlapping_InteractiveActor?`)
            (`|ExecutionSequence`
              (:`then_0`
                (`/Engine/EditorBlueprintResources/StandardMacros.DoOnce` false :!label _label_3
                  (:`Completed`
                    (message `/Game/System/Interfaces/BPI_Interactives.Overlap_Begin` (`self.Overlapping_Actor`) null))))
              (:`then_1`
                (goto _label_4 :!via `Reset`)))
            (else
              (`|ExecutionSequence`
                (:`then_0`
                  (`/Engine/EditorBlueprintResources/StandardMacros.DoOnce` false :!label _label_4
                    (:`Completed`
                      (message `/Game/System/Interfaces/BPI_Interactives.Overlap_End` (`self.Overlapping_Actor`) null)
                      (`KismetSystemLibrary.Delay` 1e-06)
                      (set `self.Overlapping_Actor` null))))
                (:`then_1`
                  (goto _label_3 :!via `Reset`))))))
        (:`then_1`
          (if (`self.Facing_InteractiveActor?`)
            (`|ExecutionSequence`
              (:`then_0`
                (`/Engine/EditorBlueprintResources/StandardMacros.DoOnce` false :!label _label_5
                  (:`Completed`
                    (message `/Game/System/Interfaces/BPI_Interactives.Facing_Begin` (`self.Facing_Actor`) null))))
              (:`then_1`
                (goto _label_6 :!via `Reset`)))
            (else
              (`|ExecutionSequence`
                (:`then_0`
                  (`/Engine/EditorBlueprintResources/StandardMacros.DoOnce` false :!label _label_6
                    (:`Completed`
                      (message `/Game/System/Interfaces/BPI_Interactives.Facing_End` (`self.Facing_Actor`) null)
                      (`KismetSystemLibrary.Delay` 1e-06)
                      (set `self.Facing_Actor` null))))
                (:`then_1`
                  (goto _label_5 :!via `Reset`))))))
        (:`then_2`
          (if (`self.Looking_InteractiveActor?`)
            (`|ExecutionSequence`
              (:`then_0`
                (`/Engine/EditorBlueprintResources/StandardMacros.DoOnce` false :!label _label_7
                  (:`Completed`
                    (message `/Game/System/Interfaces/BPI_Interactives.Looking_Begin` (`self.Looking_Actor`) null))))
              (:`then_1`
                (goto _label_8 :!via `Reset`)))
            (else
              (`|ExecutionSequence`
                (:`then_0`
                  (`/Engine/EditorBlueprintResources/StandardMacros.DoOnce` false :!label _label_8
                    (:`Completed`
                      (message `/Game/System/Interfaces/BPI_Interactives.Looking_End` (`self.Looking_Actor`) null)
                      (`KismetSystemLibrary.Delay` 1e-06)
                      (set `self.Looking_Actor` null))))
                (:`then_1`
                  (goto _label_7 :!via `Reset`))))))))))