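; GM_Default is the default game mode that spawns and sets up the player pawn at BeginPlay.
; A macro picks a PlayerStart tagged "PlayerStart", falling back to the first one found, then to a fixed transform near the world origin.
; It spawns BP_Playerpawn_Default there, possesses it, adds its HUD widget to the viewport, and passes pawn, controller and widget references to the pawn.
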(event EventBeginPlay
  (bind _returnvalue (Game|GetPlayerController 0))
  (|ComputePlayerPawnSpawnLocation
    (:Completed
      (bind _returnvalue_2 (Game|SpawnActorfromClass "/Game/Actors/Pawns/BP_Playerpawn_Default.BP_Playerpawn_Default_C" (Variables|Settings|PlayerPawn|GetPlayerPawn_Spawn_Transform) "Undefined" "MultiplyWithRoot" 0 0))
      (Pawn|Possess _returnvalue _returnvalue_2)
      (bind _returnvalue_3 (UserInterface|CreateWidget "/Game/Ui/WBP_PlayerPawn_Default.WBP_PlayerPawn_Default_C" _returnvalue))
      (UserInterface|Viewport|AddtoViewport _returnvalue_3 0)
      (Default|PlayerPawnData _returnvalue_2 _returnvalue_2 _returnvalue _returnvalue_3))))

(fn ConstructionScript)